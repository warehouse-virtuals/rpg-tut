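; BP_Enemy is an enemy character with an overhead-style health bar widget, driven by an AIC_Enemy controller.
; It forwards health, damage, healing and death queries to BPC_DamageSystem, and exposes patrol route, movement speed tiers and a zeroed ideal range.
; On death it enables mesh physics for a ragdoll, stops the controller's brain logic and sets the AI state to dead.
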(event OnDeath(BPC_DamageSystem)
  (bind _mesh (Variables|Character|GetMesh))
  (bind _aic_enemy (Variables|Default|GetAIC%20Enemy))
  (Physics|SetSimulatePhysics _mesh true)
  (Collision|SetCollisionEnabled _mesh "QueryAndPhysics")
  (AI|Logic|StopLogic (Variables|/Script/AIModule.AIController|GetBrainComponent _aic_enemy) "")
  (Default|SetStateasDead _aic_enemy))

(event EventBeginPlay
  (bind _asaic_enemy (Utilities|Casting|CastToAIC_Enemy (AI|GetAIController self)))
  (Variables|Default|SetAIC%20Enemy _asaic_enemy)
  (bind _returnvalue (UserInterface|CreateWidget "/Game/DamageSystem/W_HealthBar.W_HealthBar_C" 0 self))
  (UserInterface|SetWidget (Variables|Default|GetWidget) _returnvalue))

(fn ConstructionScript)

(fn GetCurrentHealth
  (return (Variables|/Game/DamageSystem/BPC_DamageSystem.BPC_DamageSystem_C|GetHealth (Variables|Default|GetBPC_DamageSystem))))

(fn GetIdealRange
  (return 0.0 0.0))

(fn GetMaximumHealth
  (return (Variables|/Game/DamageSystem/BPC_DamageSystem.BPC_DamageSystem_C|GetMaxHealth (Variables|Default|GetBPC_DamageSystem))))

(fn GetPatrolRoute
  (return (Variables|Default|GetPatrolRoute)))

(fn Heal
  (params (Amount :type Float%20%28double-precision%29))
  (bind _newhealth (Default|Heal (Variables|Default|GetBPC_DamageSystem) Amount))
  (return _newhealth))

(fn IsDead
  (return (Variables|/Game/DamageSystem/BPC_DamageSystem.BPC_DamageSystem_C|GetisDead (Variables|Default|GetBPC_DamageSystem))))

(fn SetMovementSpeed
  (params (Speed :type E_MovementSpeed%20Enum :default "NewEnumerator0"))
  (bind _output_get (Variables|/Script/Engine.CharacterMovementComponent|SetMaxWalkSpeed (Variables|Character|GetCharacterMovement) (Utilities|Select :Index Speed :NewEnumerator0 0.0 :NewEnumerator1 1e+02 :NewEnumerator2 3e+02 :NewEnumerator3 5e+02)))
  (return _output_get))

(fn TakeDamage
  (params (DamageInfo :type S%20Damage%20Info%20Structure))
  (bind _wasdamaged (Default|TakeDamage (Variables|Default|GetBPC_DamageSystem) DamageInfo))
  (return _wasdamaged))