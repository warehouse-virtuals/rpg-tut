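; Regular melee enemy that spawns a sword sheathed at its hip, attacks with a montage and supplies ideal attack and defend ranges.
; Equip and unequip montages move the sword between hand and sheath sockets on notify.
; A looping timer sphere-traces along the blade, with a DoOnce limiting player damage and impact sound until trace stop resets it.
; Damage responses halt movement, play indexed hit montages and switch AI stun and combat states.
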(event OnDamageResponse(BPC_DamageSystem)
  (params (DamageResponse :type E_DamageResponse%20Enum :default "NewEnumerator1"))
  (Components|Movement|StopMovementImmediately (Variables|Character|GetCharacterMovement))
  (Default|SetStateasStun (Variables|Default|GetAIC%20Enemy))
  (Animation|Montage|PlayMontage (Variables|Character|GetMesh) (Utilities|Array|Get(acopy) (Variables|Default|GetHitAnims) (Variables|Default|GetHitIndex))
    (:then
      (Math|Integer|IncrementInt (Variables|Default|GetHitIndex)
        (:%20%20
          (Default|SetStateasCombat (Variables|Default|GetAIC%20Enemy) 0 true))))
    (:OnCompleted
      (Variables|Default|SetHitIndex 0))))

(event Custom|StartSwordTrace
  ;[0.05098 0.05098 0.05098] Start Sword Trace
  (bind _returnvalue (Utilities|Time|SetTimerbyEvent (delegate Custom|HitControl) 0.01 true))
  (Variables|Default|SetTraceTimer _returnvalue))

(event Custom|HitControl
  (bind _weaponactor (Variables|Default|GetWeaponActor))
  (bind _item (Variables|/Game/Props/BP_Pickable.BP_Pickable_C|GetItem _weaponactor))
  ;[0.05098 0.05098 0.05098] Hit Control
  (bind _outactors (Actor|GetAllActorsOfClass "/Game/Props/BP_Pickable.BP_Pickable_C"))
  (if (Actor|ActorHasTag _weaponactor "weapon")
    (bind _outhit (Collision|SphereTraceByChannel (Transformation|GetSocketLocation _item "weapon_base") (Transformation|GetSocketLocation _item "weapon_tip") 2e+01 "TraceTypeQuery1" false _outactors "None"))
    (bind _asbp_third_person_character (Utilities|Casting|CastToBP_ThirdPersonCharacter (.hitactor _outhit)))
    (Utilities|FlowControl|DoOnce false
      (:Completed
        ;[0.05098 0.05098 0.05098] Damage Apply
        (Default|TakeDamage _asbp_third_person_character (Utilities|Struct|MakeS_DamageInfo 5e+01 "NewEnumerator1" "NewEnumerator3" false false false false))
        ;[0.05098 0.05098 0.05098] Play Sound
        (Audio|PlaySoundatLocation "/Game/Characters/Enemy/Sounds/MS_Sword.MS_Sword" (.impactpoint _outhit) "0, 0, 0" 1.0 1.0 0.0 0 0 0 0)))))

(event Custom|StopSwordTrace
  ;[0.05098 0.05098 0.05098] Stop Sword Trace
  (Utilities|Time|ClearandInvalidateTimerbyHandle (Variables|Default|GetTraceTimer))
  (CallFunction|ResetSwordDamage))

(event Custom|ResetSwordDamage
  ;[0.05098 0.05098 0.05098] Hit Control
  (Utilities|FlowControl|DoOnce false) ; enters at Reset
)

(event EventBeginPlay
  (|CallParentFunction)
  (bind _returnvalue (Game|SpawnActorfromClass "/Game/Props/Weapons/Sword/BP_Sword.BP_Sword_C" (Transformation|GetActorTransform) "Undefined" "MultiplyWithRoot" 0 0))
  (bind _output_get (Variables|Default|SetWeaponActor _returnvalue))
  (Transformation|AttachComponentToComponent _output_get (Variables|Character|GetMesh) "sheath_l_Socket" "SnapToTarget" "SnapToTarget" "SnapToTarget" true))

(event EventAttack
  (Animation|Montage|PlayMontage (Variables|Character|GetMesh) "/Game/Characters/MyCharacter/Animations/SwordAnims/Attack_Move_med_L_1_Montage.Attack_Move_med_L_1_Montage"
    (:OnCompleted
      _)
    (:OnInterrupted
      _))
  (Default|CallOnAttackEnd))

(event EventEquipWeapon
  (bind _notifyname (Animation|Montage|PlayMontage (Variables|Character|GetMesh) "/Game/Characters/Enemy/Animations/Sheathe/Wield_Montage.Wield_Montage")
    (:OnCompleted
      (Default|CallOnWieldEnd))
    (:OnNotifyBegin
      (switch name _notifyname
        (:Attach
          (Transformation|AttachComponentToComponent (Variables|Default|GetWeaponActor) (Variables|Character|GetMesh) "hand_r_Socket" "SnapToTarget" "SnapToTarget" "SnapToTarget" true)
          (Variables|Default|SetIsWieldingWeapon true))))))

(event EventUnequipWeapon
  (bind _notifyname (Animation|Montage|PlayMontage (Variables|Character|GetMesh) "/Game/Characters/Enemy/Animations/Sheathe/Sheathe_Montage.Sheathe_Montage")
    (:OnCompleted
      (Default|CallOnSheatheEnd))
    (:OnNotifyBegin
      (switch name _notifyname
        (:Attach
          (Transformation|AttachComponentToComponent (Variables|Default|GetWeaponActor) (Variables|Character|GetMesh) "sheath_l_Socket" "SnapToTarget" "SnapToTarget" "SnapToTarget" true)
          (Variables|Default|SetIsWieldingWeapon false))))))

(fn ConstructionScript
  (|CallParentFunction))

(fn GetIdealRange
  (return 175.0 3.5e+02))