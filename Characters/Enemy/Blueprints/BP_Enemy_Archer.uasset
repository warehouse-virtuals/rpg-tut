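; Archer enemy character that spawns a bow into its left hand on begin play and fights the player at range.
; Draw montage notifies spawn an arrow in the right hand and run a looping timer that snaps the bow's string bone to the hand socket.
; Attack detaches the arrow, aims it at the player and activates its projectile movement.
; It also supplies its ideal combat range and movement speed tiers.
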(event Custom|PullString
  ;[1 1 1] String Location Update
  (Components|PoseableMesh|SetBoneTransformbyName (Variables|/Game/Props/Weapons/Bow/BP_Bow.BP_Bow_C|GetBowMesh (stale EventBowDraw _asbp_bow)) "String" (Transformation|GetSocketTransform (Variables|Character|GetMesh) "hand_r_bowstring" "RTS_World") "WorldSpace"))

(event EventBowDraw
  (bind _notifyname (Animation|Montage|PlayMontage (Variables|Character|GetMesh) "/Game/Characters/Enemy/Animations/Archer/Bow_Draw_Montage.Bow_Draw_Montage")
    (:OnNotifyBegin
      (switch name _notifyname
        (:SpawnArrow
          ;[1 1 1] Spawn Arrow and Attach to Hand
          (Variables|Default|GetArrowRef
            (:then)
            (:else
              (bind _returnvalue (Game|SpawnActorfromClass "/Game/Props/Weapons/Arrow/BP_Arrow.BP_Arrow_C" (Transformation|GetWorldTransform (Variables|Character|GetMesh)) "Undefined" "MultiplyWithRoot" 0 0))
              (bind _output_get (Variables|Default|SetArrowRef _returnvalue))
              (Transformation|AttachComponentToComponent _output_get (Variables|Character|GetMesh) "hand_r_bowstring" "SnapToTarget" "SnapToTarget" "SnapToTarget" true))))
        (:PullString
          ;[1 1 1] String Location Update
          (bind _asbp_bow (Utilities|Casting|CastToBP_Bow (Variables|Default|GetWeaponActor)))
          (bind _returnvalue_2 (Utilities|Time|SetTimerbyEvent (delegate Custom|PullString) 0.01 true))
          (Variables|Default|SetStringPullTimerRef _returnvalue_2))
        (:EndPullString
          ;[1 1 1] String Location Update End
          (Utilities|Time|ClearandInvalidateTimerbyHandle (Variables|Default|GetStringPullTimerRef))
          (Default|CallOnBowDrawEnd))))))

(event EventEquipWeapon
  (bind _returnvalue (Game|SpawnActorfromClass "/Game/Props/Weapons/Bow/BP_Bow.BP_Bow_C" (Transformation|GetActorTransform) "Undefined" "MultiplyWithRoot" 0 0))
  (bind _output_get (Variables|Default|SetWeaponActor _returnvalue))
  (Transformation|AttachComponentToComponent _output_get (Variables|Character|GetMesh) "hand_l_socket" "SnapToTarget" "SnapToTarget" "SnapToTarget" true)
  (Variables|Default|SetIsWieldingWeapon true)
  (Default|CallOnWieldEnd))

(event EventBeginPlay
  (|CallParentFunction)
  (CallFunction|EquipWeapon))

(event EventAttack
  (Transformation|DetachFromActor (Variables|Default|GetArrowRef) "KeepWorld" "KeepWorld" "KeepWorld")
  (Transformation|SetActorRotation (Variables|Default|GetArrowRef) (Math|Rotator|FindLookatRotation (Transformation|GetActorLocation (Variables|Default|GetArrowRef)) (Transformation|GetActorLocation (Game|GetPlayerCharacter 0))))
  (Game|Components|ProjectileMovement|SetVelocityinLocalSpace (Variables|/Game/Props/Weapons/Arrow/BP_Arrow.BP_Arrow_C|GetProjectileMovement (Variables|Default|GetArrowRef)) (Variables|/Script/Engine.MovementComponent|GetVelocity (Variables|/Game/Props/Weapons/Arrow/BP_Arrow.BP_Arrow_C|GetProjectileMovement (Variables|Default|GetArrowRef))))
  (Components|Activation|Activate (Variables|/Game/Props/Weapons/Arrow/BP_Arrow.BP_Arrow_C|GetProjectileMovement (Variables|Default|GetArrowRef)) false)
  (Variables|Default|SetArrowRef 0)
  (Utilities|FlowControl|Delay 0.2)
  (Default|CallOnAttackEnd))

(fn ConstructionScript
  (|CallParentFunction))

(fn SetMovementSpeed
  (params (Speed :type E_MovementSpeed%20Enum :default "NewEnumerator0"))
  (bind _output_get (Variables|/Script/Engine.CharacterMovementComponent|SetMaxWalkSpeed (Variables|Character|GetCharacterMovement) (Utilities|Select :Index Speed :NewEnumerator0 0.0 :NewEnumerator1 2e+02 :NewEnumerator2 3.5e+02 :NewEnumerator3 5e+02)))
  (return _output_get))

(fn GetIdealRange
  (return 6e+02 6e+02))