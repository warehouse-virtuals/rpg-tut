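; BP_PatrolRoute defines an enemy patrol path as a spline, with each spline point serving as a waypoint.
; It tracks a current RouteIndex and returns that point's world location through WorldLocationOfSplinePoint.
; IncrementPatrolRouteIndex steps the index by Direction and flips it at either end, so the route ping-pongs instead of looping.
; The index and direction live on the route itself.
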(event Custom|IncrementPatrolRouteIndex
  (bind _output_get (Variables|Default|SetRoute%20Index (+ (Variables|Default|GetRoute%20Index) (Variables|Default|GetDirection))))
  (if (== _output_get (- (Spline|GetNumberOfSplinePoints (Variables|Default|GetPatrolRoute)) 1))
    (Variables|Default|SetDirection -1)
    (elif (== (Variables|Default|GetRoute%20Index) 0)
      (Variables|Default|SetDirection 1))))

(fn ConstructionScript)

(fn WorldLocationOfSplinePoint
  (return (Spline|GetLocationatSplinePoint (Variables|Default|GetPatrolRoute) (Variables|Default|GetRoute%20Index) "World")))